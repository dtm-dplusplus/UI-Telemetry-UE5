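; Enemy turret pawn Blueprint that sets up Toon telemetry for the projectiles it fires.
; On BeginPlay it creates a projectile telemetry instance named after the turret, with custom columns.
; Fire binds each projectile's hit event, whose handler builds a string list from the projectile's location and the hit actor's name.
; The logging is unfinished: neither that list nor fire-time location data reaches the telemetry instance.
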(event Custom|OnActorHit_Event
  (params (SelfActor :type Actor%20Object%20Reference) (OtherActor :type Actor%20Object%20Reference) (NormalImpulse :type Vector) (Hit :type Hit%20Result%20Structure%20%28by%20ref%29))
  ;[1 1 1] On Fire we get the projectile fire and hit event data
  (Utilities|Array|Add (Class|ToonTelemetryHelper|GetVectortoStringList (Transformation|GetActorLocation SelfActor)) (Utilities|GetDisplayName OtherActor)))

(event EventFire
  (params (ProjectileFired :type Toon%20Projectile%20Object%20Reference))
  ;[1 1 1] On Fire we get the projectile fire and hit event data
  (Collision|AssignOnActorHit ProjectileFired (delegate Custom|OnActorHit_Event)))

(event EventBeginPlay
  ;[1 1 1] Setup our telemetry instances
  (bind _returnvalue (Class|ToonTelemetrySubsystem|CreateTelemetryInstance (Subsystems|GetToonTelemetrySubsystem) (Utilities|String|Append (Utilities|GetObjectName self) "Projectiles") (Variables|Default|GetProjectileTelemetryColums)))
  (Variables|Default|SetProjectileTelemetry _returnvalue))

(fn ConstructionScript)