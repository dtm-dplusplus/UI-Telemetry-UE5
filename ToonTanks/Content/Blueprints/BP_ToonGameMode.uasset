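; BP_ToonGameMode is a game mode Blueprint that decides when the game ends and whether it is won.
; ActorDied calls IsGameOver, which sets GameWon to true when EnemiesAliveCount is zero, otherwise to false if the player died.
; When the game is over, it broadcasts OnGameOver with the result.
; GameStart is an empty event, and the enemy count is only read here, never updated.
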(event EventGameStart)

(event EventActorDied
  (params (bIsPlayer :type Boolean))
  (bind _isgameover (CallFunction|IsGameOver bIsPlayer))
  (if _isgameover
    (Default|CallOnGameOver (Variables|Default|GetbGameWon))))

(fn ConstructionScript)

(fn IsGameOver
  (params (IsPlayerDead :type Boolean))
  ;[1 1 1] Check if the game is over. True if all enemies or the player is dead. If GameOver we set the value of gamewon
  (if (== (Variables|Default|GetEnemiesAliveCount) 0)
    (Variables|Default|SetbGameWon true)
    (elif IsPlayerDead
      (Variables|Default|SetbGameWon false)
      (else
        (return false))))
  (return true))