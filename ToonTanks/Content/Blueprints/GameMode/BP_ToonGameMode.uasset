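; Game mode for the Toon game that decides when a match is won or lost and shows the end screen.
; On each actor death it checks for a win at zero living enemies first, then for a loss if the player died.
; Game over fires a delegate, then swaps the "Game" UI layer's active widget for UI_EndGame with the result message.
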(event Custom|OnGameOver
  (params (bWonGame :type Boolean))
  (bind _returnvalue (Subsystems|GetToonUISubsystem))
  (Class|ToonUISubsystem|RemoveActiveWidgetbyLayerName _returnvalue "Game")
  (bind _returnvalue_2 (Class|ToonUISubsystem|PushWidgetbyLayerName _returnvalue "/Game/UI/Pages/UI_EndGame.UI_EndGame_C" "Game"))
  (bind _asui_end_game (Utilities|Casting|CastToUI_EndGame _returnvalue_2))
  (Default|SetGameOverMessage _asui_end_game (select (Variables|Default|GetbGameWon) "You Win!!" "You Loose!")))

(event EventBeginPlay)

(event EventActorDied
  (params (bIsPlayer :type Boolean))
  (bind _bgamewon (Variables|Default|GetbGameWon))
  (bind _isgameover (CallFunction|IsGameOver bIsPlayer))
  (if _isgameover
    (Default|CallOnGameOverDelegate _bgamewon)
    (CallFunction|OnGameOver _bgamewon)))

(fn ConstructionScript)

(fn IsGameOver
  (params (IsPlayerDead :type Boolean))
  ;[1 1 1] Check if the game is over. True if all enemies or the player is dead. If GameOver we set the value of gamewon
  (if (== (Variables|Default|GetEnemiesAliveCount) 0)
    (Variables|Default|SetbGameWon true)
    (elif IsPlayerDead
      (Variables|Default|SetbGameWon false)
      (else
        (return false))))
  (return true))